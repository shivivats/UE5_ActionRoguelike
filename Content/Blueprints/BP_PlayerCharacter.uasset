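; BP_PlayerCharacter is the player character Blueprint, adding health display widgets and Parry input.
; On BeginPlay it creates a WBP_MinionHealth widget attached to itself, reusing the minion health display above the player.
; AttributeComp health changes print the new health and spawn a WBP_HealthChangePopUp widget showing the delta.
; The Parry input starts the "Parry" action by name through ActionComp.
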(event `self.ReceiveBeginPlay`
  (bind _returnvalue (`|CreateWidget` "/Game/UI/WBP_MinionHealth.WBP_MinionHealth_C" null self)) ; Can use the MinionHealth here sicne its not tied to the minion specificallty, its just to show health on top of a character
  (`UserWidget.AddToViewport` _returnvalue 0))

(event `self.AttributeComp.OnHealthChanged`
  (params (InstigatorActor :type "Actor Object Reference") (OwningComp :type "SAttributeComponent Object Reference") (NewHealth :type "Float (single-precision)") (Delta :type "Float (single-precision)"))
  (`KismetSystemLibrary.PrintString` (`KismetStringLibrary.Conv_DoubleToString` NewHealth) true false (struct :`R` 1.0 :`G` 0.512465 :`B` 0.077199 :`A` 1.0))
  (bind _returnvalue (`|CreateWidget` "/Game/UI/WBP_HealthChangePopUp.WBP_HealthChangePopUp_C" null self Delta))
  (`UserWidget.AddToViewport` _returnvalue 0))

(event `InputAction|Parry`
  (params (Key :type "Key Structure"))
  (:`Pressed`
    (`SActionComponent.StartActionByName` (`self.ActionComp`) self "Parry")))

(fn `UserConstructionScript`)