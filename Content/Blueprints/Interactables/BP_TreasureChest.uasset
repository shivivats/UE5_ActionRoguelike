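; BP_TreasureChest is an interactable chest that toggles open and closed when used by a pawn holding the required keycard gameplay tag.
; Interact checks the instigator's SActionComponent active tags, then a FlipFlop plays or reverses a timeline that drives the lid mesh's pitch.
; Gold particles activate when the timeline finishes on an opening.
; Without the tag, it prints the missing tag name as debug text.
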(event `SGameplayInterface.Interact`
  (params (InstigatorPawn :type "Pawn Object Reference"))
  (if (`BlueprintGameplayTagLibrary.HasTag` (`SActionComponent.ActiveGameplayTags` (`self.GetComponentByClass` InstigatorPawn "/Script/ActionRoguelike.SActionComponent")) (`self.RequiredKeyCard`))
    (bind _isa (`/Engine/EditorBlueprintResources/StandardMacros.FlipFlop`)
      (:`A`
        (bind (_direction _pitch) (`Timeline|AnimateLid` :!label _label)
          (:`Update`
            (`SceneComponent.K2_SetRelativeRotation` (`self.LidMesh`) (`KismetMathLibrary.MakeRotator` 0.0 _pitch) false false))
          (:`Finished`
            (if _isa
              (`ActorComponent.Activate` (`self.GoldParticles`) false)))))
      (:`B`
        (goto _label :!via `Reverse`)))
    (else
      (`KismetSystemLibrary.PrintString` (`KismetStringLibrary.Concat_StrStr` "Missing Tag: " (`BlueprintGameplayTagLibrary.GetDebugStringFromGameplayTag` (`self.RequiredKeyCard`))) true true (struct :`R` 0.609375 :`B` 0.067883 :`A` 1.0)))))

(fn `UserConstructionScript`)