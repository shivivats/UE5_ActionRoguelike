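; Sprint action that raises the instigator's movement speed while it is active.
; StartAction calls the parent implementation, then adds BonusSpeed to MaxWalkSpeed on the instigator's CharacterMovementComponent.
; StopAction calls the parent, then subtracts the same BonusSpeed, so the change is relative rather than restoring a cached original value.
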(event `self.StartAction`
  (params (Instigator :type "Actor Object Reference"))
  (bind _returnvalue (`Actor.GetComponentByClass` Instigator "/Script/Engine.CharacterMovementComponent"))
  (`parent.StartAction` Instigator) ; Be sure to call super in BlueprintNativeEvents
  (set `CharacterMovementComponent.MaxWalkSpeed` (+ (`CharacterMovementComponent.MaxWalkSpeed` _returnvalue) (`self.BonusSpeed`)) _returnvalue))

(event `self.StopAction`
  (params (Instigator :type "Actor Object Reference"))
  (bind _returnvalue (`Actor.GetComponentByClass` Instigator "/Script/Engine.CharacterMovementComponent"))
  (`parent.StopAction` Instigator) ; Be sure to call super in BlueprintNativeEvents
  (set `CharacterMovementComponent.MaxWalkSpeed` (- (`CharacterMovementComponent.MaxWalkSpeed` _returnvalue) (`self.BonusSpeed`)) _returnvalue))